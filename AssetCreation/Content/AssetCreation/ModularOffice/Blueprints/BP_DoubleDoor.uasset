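; BP_DoubleDoor is a double door that swings open when the player character enters its Box trigger and closes when the player leaves.
; Begin overlap plays the DoubleDoorOpen timeline from the start, while end overlap runs a separate timeline in reverse from the end.
; Both timelines lerp the relative yaw of BPDoor and BPDoorMirror between a shared closed angle and each leaf's own open angle.
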(event `self.Box.OnComponentBeginOverlap`
  (params (OverlappedComponent :type "PrimitiveComponent Object Reference") (OtherActor :type "Actor Object Reference") (OtherComp :type "PrimitiveComponent Object Reference") (OtherBodyIndex :type Integer) (bFromSweep :type Boolean) (SweepResult :type "HitResult Structure (by ref)"))
  (if (== OtherActor (`GameplayStatics.GetPlayerCharacter` 0))
    (bind (_direction _dooropen) (`Timeline|DoubleDoorOpen` :!via `PlayFromStart`)
      (:`Update`
        (`SceneComponent.K2_SetRelativeRotation` (`self.BP_Door`) (`KismetMathLibrary.MakeRotator` 0.0 0.0 (`KismetMathLibrary.Lerp` (`self.DoorClosed`) (`self.DoorOpen`) _dooropen)) false false)
        (`SceneComponent.K2_SetRelativeRotation` (`self.BP_DoorMirror`) (`KismetMathLibrary.MakeRotator` 0.0 0.0 (`KismetMathLibrary.Lerp` (`self.DoorClosed`) (`self.MirrorDoorOpen`) _dooropen)) false false)))))

(event `self.Box.OnComponentEndOverlap`
  (params (OverlappedComponent :type "PrimitiveComponent Object Reference") (OtherActor :type "Actor Object Reference") (OtherComp :type "PrimitiveComponent Object Reference") (OtherBodyIndex :type Integer))
  (if (== OtherActor (`GameplayStatics.GetPlayerCharacter` 0))
    (bind (_direction _dooropen) (`Timeline|Timeline` :!via `ReverseFromEnd`)
      (:`Update`
        (`SceneComponent.K2_SetRelativeRotation` (`self.BP_Door`) (`KismetMathLibrary.MakeRotator` 0.0 0.0 (`KismetMathLibrary.Lerp` (`self.DoorClosed`) (`self.DoorOpen`) _dooropen)) false false)
        (`SceneComponent.K2_SetRelativeRotation` (`self.BP_DoorMirror`) (`KismetMathLibrary.MakeRotator` 0.0 0.0 (`KismetMathLibrary.Lerp` (`self.DoorClosed`) (`self.MirrorDoorOpen`) _dooropen)) false false)))))

(fn `UserConstructionScript`)